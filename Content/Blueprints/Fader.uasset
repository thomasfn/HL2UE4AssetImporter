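; Fader is a reusable utility that drives a normalized fade value between 0 and 1 over a given duration.
; FadeIn and FadeOut set a signed speed that Tick integrates, clamping at the limits and calling the matching completion callback.
; A non-positive duration snaps straight to the end value without firing that callback.
; Helpers expose the value, the fade direction, and float or vector interpolation driven by it.
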(event `Tick`
  (params (deltaTime :type "Float (double-precision)"))
  (bind _returnvalue (+ (`self.currentFadeValue`) (* deltaTime (`self.currentFadeSpeed`))))
  (if (and (>= _returnvalue 1.0) (`self.IsFadingIn`))
    (set `self.currentFadeSpeed` 0.0)
    (set `self.currentFadeValue` 1.0)
    (`self.OnFadeInComplete`)
    (elif (and (<= _returnvalue 0.0) (`self.IsFadingOut`))
      (set `self.currentFadeSpeed` 0.0)
      (set `self.currentFadeValue` 0.0)
      (`self.OnFadeOutComplete`)
      (else
        (set `self.currentFadeValue` _returnvalue)))))

(event `FadeIn`
  (params (duration :type "Float (double-precision)"))
  (if (<= duration 0.0)
    (set `self.currentFadeSpeed` 0.0)
    (set `self.currentFadeValue` 1.0)
    (else
      (set `self.currentFadeSpeed` (/ 1.0 duration)))))

(event `FadeOut`
  (params (duration :type "Float (double-precision)"))
  (if (<= duration 0.0)
    (set `self.currentFadeSpeed` 0.0)
    (set `self.currentFadeValue` 0.0)
    (else
      (set `self.currentFadeSpeed` (/ -1.0 duration)))))

(fn `FadeFloat`
  (params (min :type "Float (double-precision)") (max :type "Float (double-precision)"))
  (returns (value :type "Float (double-precision)"))
  (return (`KismetMathLibrary.Lerp` min max (`self.GetFadeValue`))))

(fn `FadeVector`
  (params (min :type "Vector Structure") (max :type "Vector Structure"))
  (returns (value :type "Vector Structure"))
  (return (`KismetMathLibrary.VLerp` min max (`self.GetFadeValue`))))

(fn `GetFadeValue`
  (returns (fadeValue :type "Float (double-precision)"))
  (return (`self.currentFadeValue`)))

(fn `IsFadingIn`
  (returns (isFadingIn :type Boolean))
  (return (> (`self.currentFadeSpeed`) 0.0)))

(fn `IsFadingOut`
  (returns (isFadingIn :type Boolean))
  (return (< (`self.currentFadeSpeed`) 0.0)))