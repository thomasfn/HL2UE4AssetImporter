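; Half-Life 2 style player character Blueprint that handles sprinting and footstep audio.
; Sprint events toggle the sprint state on the HL2 character movement component.
; That component's footstep event selects a left or right tile step sound, with surface fixed to tile and strength as volume.
; Each name is looked up in the HL2 game sounds manifest, then restarted on a single footstep sound controller.
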(event `self.ReceiveBeginPlay`)

(event `BeginSprint`
  (bind _ashl2character_movement_component (cast `HL2CharacterMovementComponent` (`self.CharacterMovement`)))
  (`HL2CharacterMovementComponent.SetSprinting` _ashl2character_movement_component true))

(event `EndSprint`
  (bind _ashl2character_movement_component (cast `HL2CharacterMovementComponent` (`self.CharacterMovement`)))
  (`HL2CharacterMovementComponent.SetSprinting` _ashl2character_movement_component false))

(event `self.CharacterMovement.OnFootstep`
  (params (footstep :type "HL2Footstep Structure (by ref)"))
  (switch `EHL2FootstepType` footstep_Type
    (:`LeftStep`
      (`self.PlayFootstep` "Tile.StepLeft" footstep_Strength))
    (:`RightStep`
      (`self.PlayFootstep` "Tile.StepRight" footstep_Strength))))

(event `PlayFootstep`
  (params (soundScriptName :type Name) (volume :type "Float (double-precision)" :default 1.0))
  (bind _footstepsoundcontroller (`self.FootstepSoundController`))
  (bind (_outsuccess _returnvalue) (`HL2Utils.TryResolveHL2Script` "game_sounds_manifest"))
  (if _outsuccess
    (bind _ashl2sound_scripts (cast `HL2SoundScripts` _returnvalue))
    (`|ExecutionSequence`
      (:`then_0`
        (bind (_outsoundscript _returnvalue_2) (`HL2SoundScripts.LookupSoundScript` _ashl2sound_scripts soundScriptName))
        (if _returnvalue_2
          (`/HL2AssetImporter/Entities/Components/SoundScriptController.Stop` _footstepsoundcontroller)
          (set `/HL2AssetImporter/Entities/Components/SoundScriptController.SoundScript` _outsoundscript _footstepsoundcontroller)
          (`/HL2AssetImporter/Entities/Components/SoundScriptController.SetVolume` _footstepsoundcontroller volume)
          (`/HL2AssetImporter/Entities/Components/SoundScriptController.Play` _footstepsoundcontroller 0.0))))))

(fn `UserConstructionScript`)