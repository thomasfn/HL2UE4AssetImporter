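; Player controller for an HL2-style character that turns player input into movement and look on the controlled pawn.
; Each tick it adds movement input along forward and right vectors built from control yaw only, scaled by the forward and right axes.
; Mouse axes drive yaw and inverted pitch.
; Jump and crouch forward press and release to the pawn as a Character, while sprint calls begin and end on HL2PlayerCharacter.
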(event `self.ReceiveBeginPlay`
  (`self.ResetIgnoreMoveInput`))

(event `self.ReceiveTick`
  (params (DeltaSeconds :type "Float (single-precision)"))
  (bind (_returnvalue_roll _returnvalue_pitch _returnvalue_yaw) (`KismetMathLibrary.BreakRotator` (`self.GetControlRotation`)))
  (bind _returnvalue (`KismetMathLibrary.MakeRotator` 0.0 0.0 _returnvalue_yaw))
  (`parent.ReceiveTick` DeltaSeconds)
  (`Pawn.AddMovementInput` (`self.K2_GetPawn`) (+ (* (`KismetMathLibrary.GetForwardVector` _returnvalue) (`self.GetInputAxisValue`)) (* (`KismetMathLibrary.GetRightVector` _returnvalue) (`self.GetInputAxisValue`))) 1.0 false))

(event `InputAxisKey|MouseX`
  (params (AxisValue :type "Float (single-precision)"))
  (`self.AddYawInput` AxisValue))

(event `InputAxisKey|MouseY`
  (params (AxisValue :type "Float (single-precision)"))
  (`self.AddPitchInput` (* AxisValue -1.0)))

(event `InputAction|Jump`
  (params (Key :type "Key Structure"))
  (bind _returnvalue (`self.K2_GetPawn`))
  (:`Pressed`
    (bind _ascharacter (cast `Character` _returnvalue))
    (`Character.Jump` _ascharacter))
  (:`Released`
    (bind _ascharacter_2 (cast `Character` _returnvalue))
    (`Character.StopJumping` _ascharacter_2)))

(event `InputAction|Crouch`
  (params (Key :type "Key Structure"))
  (bind _returnvalue (`self.K2_GetPawn`))
  (:`Pressed`
    (bind _ascharacter (cast `Character` _returnvalue))
    (`Character.Crouch` _ascharacter))
  (:`Released`
    (bind _ascharacter_2 (cast `Character` _returnvalue))
    (`Character.UnCrouch` _ascharacter_2)))

(event `InputAction|Sprint`
  (params (Key :type "Key Structure"))
  (bind _returnvalue (`self.K2_GetPawn`))
  (:`Pressed`
    (bind _ashl2player_character (cast `/HL2AssetImporter/Blueprints/HL2PlayerCharacter` _returnvalue))
    (`/HL2AssetImporter/Blueprints/HL2PlayerCharacter.BeginSprint` _ashl2player_character))
  (:`Released`
    (bind _ashl2player_character_2 (cast `/HL2AssetImporter/Blueprints/HL2PlayerCharacter` _returnvalue))
    (`/HL2AssetImporter/Blueprints/HL2PlayerCharacter.EndSprint` _ashl2player_character_2)))

(fn `UserConstructionScript`)