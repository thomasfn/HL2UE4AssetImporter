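; Soundscape controller that keeps one soundscape active at a time, choosing the nearest of those competing.
; Soundscapes are added to and removed from a competing set through events.
; While that set is non-empty, Tick finds the member closest to the controller's world location.
; A change of selection deactivates the previous soundscape and activates the new one, with debug prints logging changes.
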(event `self.ReceiveTick`
  (params (DeltaSeconds :type "Float (single-precision)"))
  (if (`BlueprintSetLibrary.Set_IsNotEmpty` (`self.competingSoundscapes`))
    (bind _closest (`self.GetClosestCompetingSoundscape`))
    (`self.SelectSoundscape` _closest)))

(event `AddCompetingSoundscape`
  (params (soundscape :type "/HL2AssetImporter/Entities/env_soundscape Object Reference"))
  (`BlueprintSetLibrary.Set_Add` (`self.competingSoundscapes`) soundscape)
  (`KismetSystemLibrary.PrintString` (`KismetStringLibrary.Concat_StrStr` "AddCompetingSoundscape: " (`KismetSystemLibrary.GetDisplayName` soundscape))))

(event `RemoveCompetingSoundscape`
  (params (soundscape :type "/HL2AssetImporter/Entities/env_soundscape Object Reference"))
  (`BlueprintSetLibrary.Set_Remove` (`self.competingSoundscapes`) soundscape)
  (`KismetSystemLibrary.PrintString` (`KismetStringLibrary.Concat_StrStr` "RemoveCompetingSoundscape: " (`KismetSystemLibrary.GetDisplayName` soundscape))))

(event `SelectSoundscape`
  (params (soundscape :type "/HL2AssetImporter/Entities/env_soundscape Object Reference"))
  (if (not (== soundscape (`self.selectedSoundscape`)))
    (bind _selectedsoundscape (`self.selectedSoundscape`)
      (:`then`
        (`/HL2AssetImporter/Entities/env_soundscape.DeactivateSoundscape` _selectedsoundscape))
      (:`else`
        _))
    (bind _output_get (set `self.selectedSoundscape` soundscape))
    (`/Engine/EditorBlueprintResources/StandardMacros.IsValid` _output_get
      (:`Is Valid`
        (`/HL2AssetImporter/Entities/env_soundscape.ActivateSoundscape` _output_get)
        (`KismetSystemLibrary.PrintString` (`KismetStringLibrary.Concat_StrStr` "SelectSoundscape: " (`KismetSystemLibrary.GetDisplayName` soundscape)))))))

(fn `GetClosestCompetingSoundscape`
  (returns (closest :type "/HL2AssetImporter/Entities/env_soundscape Object Reference"))
  (locals (currentClosest :type "/HL2AssetImporter/Entities/env_soundscape Object Reference") (currentDist :type "Float (double-precision)"))
  (bind _result (`BlueprintSetLibrary.Set_ToArray` (`self.competingSoundscapes`)))
  (for _array_element _result
    (`local.currentClosest`
      (:`then`
        (bind _returnvalue (`KismetMathLibrary.Vector_Distance` (`self.K2_GetComponentLocation` (`Actor.RootComponent` _array_element)) (`self.K2_GetComponentLocation`)))
        (if (< _returnvalue (`local.currentDist`))
          (set `local.currentClosest` _array_element :!label _label)
          (set `local.currentDist` _returnvalue)))
      (:`else`
        (goto _label))))
  (return (`local.currentClosest`)))