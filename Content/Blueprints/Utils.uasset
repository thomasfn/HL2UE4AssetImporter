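; Utils is a Blueprint utility library of static lookup helpers for finding key level actors.
; GetWorldSpawn returns the first Worldspawn actor found in the world, without checking that one exists.
; GetSkybox scans all StaticMeshActors for one whose display name is "Skybox", returning nothing if none matches.
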(fn `GetSkybox`
  (params (worldContextObject :type "Actor Object Reference"))
  (returns (skybox :type "StaticMeshActor Object Reference"))
  (bind _outactors (`GameplayStatics.GetAllActorsOfClass` worldContextObject "/Script/Engine.StaticMeshActor"))
  (for _array_element _outactors
    (if (== (`KismetSystemLibrary.GetDisplayName` _array_element) "Skybox")
      (return _array_element)))
  (return null))

(fn `GetWorldSpawn`
  (params (worldContextObject :type "Actor Object Reference"))
  (returns (worldSpawn :type "/HL2AssetImporter/Entities/worldspawn Object Reference"))
  (bind _outactors (`GameplayStatics.GetAllActorsOfClass` worldContextObject "/HL2AssetImporter/Entities/worldspawn.worldspawn_C"))
  (return (`|GetArrayItem` _outactors)))